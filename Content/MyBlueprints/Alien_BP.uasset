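; Player-controlled alien ship that moves along the world X axis, fires lasers and deploys an abduction actor.
; Holding Abdusir spawns an Abduzir at AbduzirP with a back-reference to the ship, and releasing destroys it.
; Tiro spawns a Laser at TiroP, rate-limited by a countdown that resets to Recover and decreases on Tick.
; SetVida adds the given amount to Vida (health) without clamping.
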(event `InputAxis|MovimentoHorizontal`
  (params (AxisValue :type "Float (single-precision)"))
  (`self.AddMovementInput` (1.0 0.0 0.0) AxisValue))

(event `InputAction|Abdusir`
  (params (Key :type "Key Structure"))
  (:`Pressed`
    (bind _returnvalue (`|SpawnActorFromClass` "/Game/MyBlueprints/Abduzir.Abduzir_C" (`SceneComponent.K2_GetComponentToWorld` (`self.AbduzirP`)) "Undefined" "OverrideRootScale" null null))
    (bind _output_get (set `self.AbduzirAC` _returnvalue))
    (set `/Game/MyBlueprints/Abduzir.myNave` self _output_get))
  (:`Released`
    (`self.K2_DestroyActor` _output_get)))

(event `InputAction|Tiro`
  (params (Key :type "Key Structure"))
  (:`Pressed`
    (if (<= (`self.contdown`) 0.0)
      (`|SpawnActorFromClass` "/Game/MyBlueprints/Laser.Laser_C" (`SceneComponent.K2_GetComponentToWorld` (`self.TiroP`)) "Undefined" "OverrideRootScale" null null)
      (set `self.contdown` (`self.recover`)))))

(event `Coltdown`
  (params (delta :type "Float (double-precision)"))
  (if (>= (`self.contdown`) 0.0)
    (set `self.contdown` (- (`self.contdown`) delta))))

(event `self.ReceiveTick`
  (params (DeltaSeconds :type "Float (single-precision)"))
  (`self.Coltdown` DeltaSeconds))

(fn `setVida`
  (params (qtd :type "Float (double-precision)"))
  (set `self.vida` (+ (`self.vida`) qtd)))

(fn `UserConstructionScript`)